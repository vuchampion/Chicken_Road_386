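; BP_Log is a moving log that travels along world X and destroys itself once past its travel limit plus half its scaled length.
; StartLog sets direction, speed and length, stretches the log and returns its scaled length.
; Player overlap begin and end both call Sink, dipping the mesh once; Unsink exists but is uncalled here.
; SetupNodes, also uncalled here, spawns evenly spaced Node actors attached along it.
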(event OnComponentEndOverlap(Box)
  (params (OverlappedComponent :type Primitive%20Component%20Object%20Reference) (OtherActor :type Actor%20Object%20Reference) (OtherComp :type Primitive%20Component%20Object%20Reference) (OtherBodyIndex :type Integer))
  (Utilities|Casting|CastToBPC_Player OtherActor)
  (CallFunction|Sink))

(event OnComponentBeginOverlap(Box)
  (params (OverlappedComponent :type Primitive%20Component%20Object%20Reference) (OtherActor :type Actor%20Object%20Reference) (OtherComp :type Primitive%20Component%20Object%20Reference) (OtherBodyIndex :type Integer) (bFromSweep :type Boolean) (SweepResult :type Hit%20Result%20Structure%20%28by%20ref%29))
  (Utilities|Casting|CastToBPC_Player OtherActor)
  (CallFunction|Sink))

(event EventBeginPlay)

(event Collision|EventActorBeginOverlap
  (params (OtherActor :type Actor%20Object%20Reference)))

(event EventTick
  (params (DeltaSeconds :type Float%20%28single-precision%29))
  (bind _move_speed (Variables|Default|GetMove_Speed))
  (if (>= (+ (/ (* (Variables|Default|GetLength) (Variables|Default|GetScale)) 2.0) (Variables|Default|GetMaxTravel)) (Variables|Default|GetTraveled))
    (Transformation|AddActorWorldOffset (Math|Vector|MakeVector (* (Variables|Default|GetDirection) _move_speed) 0.0 0.0) true)
    (Variables|Default|SetTraveled (+ _move_speed (Variables|Default|GetTraveled)))
    (else
      (Actor|DestroyActor))))

(fn ConstructionScript)

(fn StartLog
  (params (Direction :type Integer) (MoveSpeed :type Float%20%28single-precision%29) (Length :type Integer))
  (Variables|Default|SetDirection Direction)
  (CallFunction|RotateLog)
  (Variables|Default|SetMove_Speed MoveSpeed)
  (bind _output_get (Variables|Default|SetLength Length))
  (CallFunction|StretchLog)
  (return (* _output_get (Variables|Default|GetScale))))

(fn Sink
  (if (not (Variables|Default|GetSunk))
    (Transformation|AddWorldOffset (Variables|Default|GetLog) "0, 0,-5.000000" true false)
    (Variables|Default|SetSunk true)))

(fn Unsink
  (if (Variables|Default|GetSunk)
    (Transformation|AddWorldOffset (Variables|Default|GetLog) "0, 0,5.000000" true false)
    (Variables|Default|SetSunk false)))

(fn StretchLog
  (Class|Actor|AddActorLocalTransform (Math|Transform|MakeTransform "0, 0, 0" "0, 0, 0" (Math|Vector|MakeVector 1.0 (Math|Conversions|ToFloat(Integer) (/ (Variables|Default|GetLength) 2)) 1.0)) false false))

(fn RotateLog
  (if (== (Variables|Default|GetDirection) 0)
    (Variables|Default|SetDirection -1)))

(fn SetupNodes
  (bind _length (Variables|Default|GetLength))
  (Variables|Default|SetNodePoint (+ (Transformation|GetWorldLocation (Variables|Default|GetLog)) (Math|Vector|MakeVector (+ (* _length -55.0) 1.1e+02) 0.0 85.0)))
  (for _index (range 2 _length)
    (bind _returnvalue (Game|SpawnActorfromClass "/Game/Blueprints/Node.Node_C" (Math|Transform|MakeTransform (Variables|Default|GetNodePoint) "0, 0, 0" "1,1,1") "Undefined" 0 0))
    (Transformation|AttachActorToActor _returnvalue self "None" "KeepWorld" "KeepWorld" "KeepWorld" true)
    (Variables|Default|SetNodePoint (+ (Variables|Default|GetNodePoint) "110.000000,0.000000, 0"))))