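; VehicleSpawner fills a terrain lane with moving obstacles, spawning logs on terrain index 1 and vehicles on all others.
; SpawnInitialVehicles stores the lane's direction and terrain, sets its speed (fixed and fast for index 3, random otherwise), and spawns the first obstacle.
; Tick accumulates distance by that speed, rolling a random spawn chance at each spacing threshold.
; Each spawned obstacle's returned value pushes the counter negative, delaying the next roll.
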(event EventBeginPlay)

(event Collision|EventActorBeginOverlap
  (params (OtherActor :type Actor%20Object%20Reference)))

(event EventTick
  (params (DeltaSeconds :type Float%20%28single-precision%29))
  (CallFunction|CheckSpawn))

(fn ConstructionScript)

(fn SpawnInitialVehicles
  (params (Direction :type Integer) (Terrain :type Terrain%20Object%20Reference) (TerrainIndex :type Integer))
  (bind _defaultsceneroot (Variables|Default|GetDefaultSceneRoot))
  (bind _returnvalue (Transformation|GetWorldLocation _defaultsceneroot))
  (Variables|Default|SetTerrainIndex TerrainIndex)
  (Variables|Default|SetDirection Direction)
  (Variables|Default|SetTerrain Terrain)
  (CallFunction|PrepSpeed)
  (if (!= (Variables|Default|GetTerrainIndex) 1)
    (CallFunction|SpawnVehicle _returnvalue)
    (else
      (CallFunction|SpawnLog _returnvalue))))

(fn SpawnVehicle
  (params (Location :type Vector))
  (bind _returnvalue (Game|SpawnActorfromClass "/Game/Blueprints/Vehicle.Vehicle_C" (Math|Transform|MakeTransform Location "0, 0, 0" "1,1,1") "Undefined" 0 0))
  (bind _output_get (Variables|Default|SetLastVehicle _returnvalue))
  (bind _vehiclelength (Default|PrepVehicle _output_get (Variables|Default|GetTerrainIndex) (Variables|Default|GetDirection) Location self (Variables|Default|GetVehicleSpeed)))
  (Variables|Default|SetDistance (- 0.0 _vehiclelength)))

(fn PrepSpeed
  (if (== (Variables|Default|GetTerrainIndex) 3)
    (Variables|Default|SetVehicleSpeed 1.1e+02)
    (Variables|Default|SetRate 600)
    (else
      (Variables|Default|SetVehicleSpeed (Math|Random|RandomFloatinRange 5.0 1e+01))
      (Variables|Default|SetRate 60))))

(fn CheckSpawn
  (bind _defaultsceneroot (Variables|Default|GetDefaultSceneRoot))
  (bind _returnvalue (Transformation|GetWorldLocation _defaultsceneroot))
  (if (>= (Variables|Default|GetDistance) 2.2e+02)
    (Variables|Default|SetDistance 0.0)
    (if (<= 6e+01 (Math|Random|RandomFloatinRange 0.0 1e+02))
      (if (!= (Variables|Default|GetTerrainIndex) 1)
        (CallFunction|SpawnVehicle _returnvalue)
        (else
          (CallFunction|SpawnLog _returnvalue))))
    (else
      (Variables|Default|SetDistance (+ (Variables|Default|GetDistance) (Variables|Default|GetVehicleSpeed))))))

(fn SpawnLog
  (params (Location :type Vector))
  (bind _returnvalue (Game|SpawnActorfromClass "/Game/Blueprints/BP_Log.BP_Log_C" (Math|Transform|MakeTransform Location "0, 0, 0" "1,1,1") "Undefined" 0 0))
  (bind _loglength (Default|StartLog _returnvalue (Variables|Default|GetDirection) (Variables|Default|GetVehicleSpeed) (Math|Random|RandomIntegerinRange 2 5)))
  (Variables|Default|SetDistance (- 0.0 _loglength)))