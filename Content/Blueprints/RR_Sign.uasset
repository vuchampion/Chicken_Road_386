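; Railroad crossing sign that flashes two rect lights alternately and sounds a train warning when toggled on.
; ToggleActive either blanks both lights or activates the sign, starts the flash and spawns the sound at its location.
; While Active, Tick uses latent Delays as repeating timers to call SwitchLight.
; A longer delayed check calls ToggleActive if Active is false by then, switching the sign back on.
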(event EventBeginPlay)

(event Collision|EventActorBeginOverlap
  (params (OtherActor :type Actor%20Object%20Reference)))

(event EventTick
  (params (DeltaSeconds :type Float%20%28single-precision%29))
  (bind _active (Variables|Default|GetActive))
  (if _active
    (Utilities|FlowControl|Delay 0.38)
    (CallFunction|SwitchLight)
    (Utilities|FlowControl|Delay 2.0)
    (if (not _active)
      (CallFunction|ToggleActive))))

(fn ConstructionScript)

(fn ToggleActive
  (if (Variables|Default|GetActive)
    (Rendering|Components|Light|SetIntensity (Variables|Default|GetRectLight) 0.0)
    (Rendering|Components|Light|SetIntensity (Variables|Default|GetRectLight1) 0.0)
    (Variables|Default|SetActive false)
    (else
      (Variables|Default|SetSwitch true)
      (Variables|Default|SetActive true)
      (CallFunction|SwitchLight)
      (Audio|SpawnSoundatLocation "/Game/Sounds/TrainWarning.TrainWarning" (Transformation|GetWorldLocation (Variables|Default|GetDefaultSceneRoot)) "0, 0, 0" 1.0 1.0 0.0 0 0))))

(fn SwitchLight
  (bind _rectlight (Variables|Default|GetRectLight))
  (bind _rectlight1 (Variables|Default|GetRectLight1))
  (if (Variables|Default|GetActive)
    (if (Variables|Default|GetSwitch)
      (Rendering|Components|Light|SetIntensity _rectlight 0.0)
      (Rendering|Components|Light|SetIntensity _rectlight1 5e+03)
      (Variables|Default|SetSwitch false)
      (else
        (Rendering|Components|Light|SetIntensity _rectlight1 0.0)
        (Rendering|Components|Light|SetIntensity _rectlight 5e+03)
        (Variables|Default|SetSwitch true)))))