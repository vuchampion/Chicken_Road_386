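; Lilypad movement Blueprint that spins its static mesh around the yaw axis, alternating direction.
; Tick applies a frame-rate independent rotation from the truncated MaxSpeed multiplied by Offset.
; A looping timer started at BeginPlay calls ChangeOffset every few seconds to flip the sign of Offset.
; Increment and Decrement timer nodes are left unconnected and never run.
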(event Custom|Change%20Direction
  (CallFunction|ChangeOffset))

(event EventBeginPlay
  (Utilities|Time|SetTimerbyEvent (delegate Custom|Change%20Direction) 4.0 true))

(event Collision|EventActorBeginOverlap
  (params (OtherActor :type Actor%20Object%20Reference)))

(event EventTick
  (params (DeltaSeconds :type Float%20%28single-precision%29))
  (Transformation|AddWorldRotation (Variables|Default|GetStaticMesh) (Math|Rotator|MakeRotator 0.0 0.0 (* DeltaSeconds (Math|Conversions|ToFloat(Integer) (* (Math|Float|Truncate (Variables|Default|GetMax_Speed)) (Variables|Default|GetOffset))))) false false))

(fn ConstructionScript)

(fn ChangeOffset
  (Variables|Default|SetOffset (* (Variables|Default|GetOffset) -1)))